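; LootItem_Bp is a dropped loot pickup whose sphere is colored by item rarity in the construction script.
; On BeginPlay it pops out with a randomized impulse, then after a fixed delay stops simulating physics and enables query-and-physics collision.
; It then copies loot score and item stats from ItemDetails into its LootUMG widget.
; Look-at events show that widget with its world rotation zeroed, or hide it.
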(event Custom|LookAtItem
  (bind _lootumg (Variables|Default|GetLootUMG))
  (Rendering|SetVisibility _lootumg true false)
  (Transformation|SetWorldRotation _lootumg "0, 0, 0" false false))

(event Custom|StoplookingItemStats
  (Rendering|SetVisibility (Variables|Default|GetLootUMG) false false))

(event EventBeginPlay
  (bind _itemdetails (Variables|Default|GetItemDetails))
  (bind (_rarity _lootscore _itemstats) (Utilities|Struct|BreakItemStruct _itemdetails))
  (bind (_damage _accuracy _firerate _reloadspeed _magazinesize _description) (Utilities|Struct|BreakStatStruct _itemstats))
  (Physics|AddImpulse (Variables|Default|GetSphere) (* (Math|Vector|MakeVector (Math|Random|RandomFloatinRange -0.24 0.1) (Math|Random|RandomFloatinRange -0.5 -1.2) 0.0) (Variables|Default|GetLootJumpStrength)) "None" false)
  (Utilities|FlowControl|Delay 4.0)
  (Physics|SetSimulatePhysics (Variables|Default|GetSphere) false)
  (Collision|SetCollisionEnabled (Variables|Default|GetSphere) "QueryAndPhysics")
  (bind _asloot_interface (Utilities|Casting|CastToLootInterface (UserInterface|GetUserWidgetObject (Variables|Default|GetLootUMG))))
  (Variables|/Game/Loot/LootInterface.LootInterface_C|SetLootScore _asloot_interface _lootscore)
  (Variables|/Game/Loot/LootInterface.LootInterface_C|SetDMG_V _asloot_interface _damage)
  (Variables|/Game/Loot/LootInterface.LootInterface_C|SetFRR_V _asloot_interface _firerate)
  (Variables|/Game/Loot/LootInterface.LootInterface_C|SetMAG_V _asloot_interface _magazinesize)
  (Variables|/Game/Loot/LootInterface.LootInterface_C|SetACC_V _asloot_interface _accuracy)
  (Variables|/Game/Loot/LootInterface.LootInterface_C|SetRLD_V _asloot_interface _reloadspeed)
  (Variables|/Game/Loot/LootInterface.LootInterface_C|SetDES_V _asloot_interface _description))

(fn ConstructionScript
  (Rendering|Material|SetMaterial (Variables|Default|GetSphere) 0 (Utilities|Select :Index (.Rarity (Utilities|Struct|BreakItemStruct (Variables|Default|GetItemDetails))) :NewEnumerator0 "/Game/Loot/Material/LR_Grey.LR_Grey" :NewEnumerator1 "/Game/Loot/Material/LR_Blue.LR_Blue" :NewEnumerator2 "/Game/Loot/Material/LR_Violet.LR_Violet" :NewEnumerator3 "/Game/Loot/Material/LR_Red.LR_Red" :NewEnumerator4 "/Game/Loot/Material/LR_Yellow.LR_Yellow")))