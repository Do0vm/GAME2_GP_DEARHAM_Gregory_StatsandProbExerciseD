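; BP_Bullet is a short-lived gun bullet actor that destroys itself 0.1 seconds after spawning.
; When its capsule overlaps an actor without the "Ignore" tag, it applies random integer damage between the truncated BulletDamage and a fixed high maximum, then plays a 2D hit sound.
; A delayed destroy also follows the hit, but the shorter spawn timer removes the bullet first.
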(event OnComponentBeginOverlap(Capsule)
  (params (OverlappedComponent :type Primitive%20Component%20Object%20Reference) (OtherActor :type Actor%20Object%20Reference) (OtherComp :type Primitive%20Component%20Object%20Reference) (OtherBodyIndex :type Integer) (bFromSweep :type Boolean) (SweepResult :type Hit%20Result%20Structure%20%28by%20ref%29))
  ;[0.2865 0.07069 0.02195] ApplyDamage IgnoreSelf
  (if (not (Actor|ActorHasTag OtherActor "Ignore"))
    (Game|Damage|ApplyDamage OtherActor (Math|Conversions|ToFloat(Integer) (Math|Random|RandomIntegerinRange (Math|Float|Truncate (Variables|Default|GetBullet%20Damage)) 9999)) 0 self)
    (Audio|PlaySound2D "/Game/Sound/Guns/Rifle/Hit.Hit" 1.0 1.0 0.0 0 0)
    (Utilities|FlowControl|Delay 0.9)
    (Actor|DestroyActor)))

(event EventBeginPlay
  (Utilities|FlowControl|Delay 0.1)
  (Actor|DestroyActor))

(event Collision|EventActorBeginOverlap
  (params (OtherActor :type Actor%20Object%20Reference)))

(event EventTick
  (params (DeltaSeconds :type Float%20%28single-precision%29)))

(fn ConstructionScript)