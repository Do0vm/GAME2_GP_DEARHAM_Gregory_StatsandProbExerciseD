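; BP_Rifle is a rifle Blueprint that spawns BP_Bullet actors from shoot-point components, passing only their yaw as rotation.
; ShootingEvent fires from the centre point, activates the Niagara muzzle flash, plays a fire sound, then switches the flash off after a short delay.
; ModifierShooting makes a three-bullet volley by spawning from the right and left points, then running the centre-shot logic through the shared delay.
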(event Custom|ShootingEvent
  (bind _pointshootcentre (Variables|Default|GetPointShootCentre))
  (bind _ns_muzzleflash (Variables|Default|GetNS_MuzzleFlash))
  (bind _returnvalue (Transformation|GetWorldTransform _pointshootcentre))
  ;[0 0.08333 0.05387] BulletSpawning
  (Game|SpawnActorfromClass "/Game/MillAssets/Gun/BP_Bullet.BP_Bullet_C" (Math|Transform|MakeTransform (.location _returnvalue) (Math|Rotator|MakeRotator 0.0 0.0 (.yaw (.rotation _returnvalue))) (.scale _returnvalue)) "Undefined" "MultiplyWithRoot" 0 0)
  (Components|Activation|Activate _ns_muzzleflash true)
  (Audio|PlaySound2D "/Game/MilitaryWeapSilver/Sound/Rifle/Cues/RifleA_FireEnd_Cue.RifleA_FireEnd_Cue" 1.0 1.0 0.0 0 0)
  (Utilities|FlowControl|Delay 0.1)
  (Components|Activation|Deactivate _ns_muzzleflash))

(event Custom|ModifierShooting
  (bind _pointshootcentre (Variables|Default|GetPointShootCentre))
  (bind _ns_muzzleflash (Variables|Default|GetNS_MuzzleFlash))
  (bind _pointshootleft (Variables|Default|GetPointShootleft))
  (bind _pointshootright (Variables|Default|GetPointShootRight))
  (bind _returnvalue (Transformation|GetWorldTransform _pointshootright))
  (bind _returnvalue_2 (Transformation|GetWorldTransform _pointshootcentre))
  (bind _returnvalue_3 (Transformation|GetWorldTransform _pointshootleft))
  ;[0 0.08333 0.05387] BulletSpawning
  (Utilities|FlowControl|Sequence
    (:then_0
      (Game|SpawnActorfromClass "/Game/MillAssets/Gun/BP_Bullet.BP_Bullet_C" (Math|Transform|MakeTransform (.location _returnvalue) (Math|Rotator|MakeRotator 0.0 0.0 (.yaw (.rotation _returnvalue))) (.scale _returnvalue)) "Undefined" "MultiplyWithRoot" 0 0))
    (:then_1
      (Game|SpawnActorfromClass "/Game/MillAssets/Gun/BP_Bullet.BP_Bullet_C" (Math|Transform|MakeTransform (.location _returnvalue_3) (Math|Rotator|MakeRotator 0.0 0.0 (.yaw (.rotation _returnvalue_3))) (.scale _returnvalue_3)) "Undefined" "MultiplyWithRoot" 0 0))
    (:then_2
      (Game|SpawnActorfromClass "/Game/MillAssets/Gun/BP_Bullet.BP_Bullet_C" (Math|Transform|MakeTransform (.location _returnvalue_2) (Math|Rotator|MakeRotator 0.0 0.0 (.yaw (.rotation _returnvalue_2))) (.scale _returnvalue_2)) "Undefined" "MultiplyWithRoot" 0 0)
      (Components|Activation|Activate _ns_muzzleflash true)
      (Audio|PlaySound2D "/Game/MilitaryWeapSilver/Sound/Rifle/Cues/RifleA_FireEnd_Cue.RifleA_FireEnd_Cue" 1.0 1.0 0.0 0 0)))
  (Utilities|FlowControl|Delay 0.1)
  (Components|Activation|Deactivate _ns_muzzleflash))

(event EventBeginPlay
  (Components|Activation|Deactivate (Variables|Default|GetNS_MuzzleFlash)))

(fn ConstructionScript)