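; Exploding zombie enemy that roams random navigable points, chases the player on sight and detonates on contact.
; Pawn sensing sets CanSeePlayer, which gates the roam loop and the contact blast of damage, effects, camera shake and force feedback.
; Taking damage spawns BP_Damage and blood, and tweens the player camera's FOV.
; Death or detonation ragdolls the mesh with an impulse; only health-depleted deaths increment the game mode's kill count.
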(event OnSeePawn(ZombieSensing)
  (params (Pawn :type Pawn%20Object%20Reference))
  (if (== Pawn (Variables|Default|GetAs%20BP%20First%20Person%20Character))
    (Variables|Default|SetCanSeePlayer true)
    (Utilities|FlowControl|Sequence
      (:then_0
        (AI|AIMoveTo self "0, 0, 0" (Variables|Default|GetAs%20BP%20First%20Person%20Character) 5.0 false
          (:then
            (Utilities|FlowControl|RetriggerableDelay 3.0)
            (CallFunction|RoamingMapAI))))
      (:then_1
        (Utilities|FlowControl|DoOnce false
          (:Completed
            (Audio|PlaySoundatLocation (Variables|Default|GetChase) (Transformation|GetActorLocation) "0, 0, 0" 1.0 1.0 0.0 0 0 0 0)))))
    (else
      (Variables|Default|SetCanSeePlayer false))))

(event OnComponentHit(CapsuleComponent)
  (params (HitComponent :type Primitive%20Component%20Object%20Reference) (OtherActor :type Actor%20Object%20Reference) (OtherComp :type Primitive%20Component%20Object%20Reference) (NormalImpulse :type Vector :default "0, 0, 0") (Hit :type Hit%20Result%20Structure%20%28by%20ref%29))
  (bind _returnvalue (Transformation|GetActorForwardVector))
  (bind _mesh (Variables|Character|GetMesh))
  (bind _as_bp_first_person_character (Variables|Default|GetAs%20BP%20First%20Person%20Character))
  (bind _returnvalue_2 (* _returnvalue 5e+03))
  (if (== OtherActor _as_bp_first_person_character)
    (if (Variables|Default|GetCanSeePlayer)
      (Game|Damage|ApplyDamage _as_bp_first_person_character 2.0 0 self)
      (Effects|SpawnEmitteratLocation "/Game/StarterContent/Particles/P_Explosion.P_Explosion" (Transformation|GetActorLocation))
      (Audio|PlaySoundatLocation 0 (Transformation|GetActorLocation) "0, 0, 0" 1.0 1.0 0.0 0 0 0 0)
      (Game|Feedback|ClientPlayForceFeedback (Game|GetPlayerController 0) 0 "None" false false false)
      (Collision|SetCollisionProfileName _mesh "Ragdoll" true :!class /Script/Engine.PrimitiveComponent)
      (Physics|SetSimulatePhysics _mesh true)
      (Physics|AddImpulse _mesh (Math|Vector|MakeVector (.x _returnvalue_2) (.y _returnvalue_2) 0.0) "None" true)
      (Components|DestroyComponent (Variables|Collision|GetCapsuleComponent))
      (Game|Feedback|ClientStartCameraShake (Game|GetPlayerController 0) "/Game/MillAssets/Camera/BP_ExplosionCamera.BP_ExplosionCamera_C" 1.0 "CameraLocal" "0, 0, 0")
      (Utilities|FlowControl|Delay 4.0)
      (Actor|DestroyActor))))

(event Custom|RoamingMapAI
  (bind _randomlocation (Class|NavigationSystemV1|GetRandomLocationinNavigableRadius (Transformation|GetActorLocation) (Variables|Default|GetRadius) 0 0 :!label _label))
  (AI|AIMoveTo self _randomlocation 0 5.0 false
    (:then
      _)
    (:OnFail
      _))
  (Utilities|FlowControl|Delay (Variables|Default|GetDuration))
  (if (not (Variables|Default|GetCanSeePlayer))
    (goto _label)))

(event Game|Damage|EventAnyDamage
  (params (Damage :type Float%20%28single-precision%29) (DamageType :type Damage%20Type%20Object%20Reference) (InstigatedBy :type Controller%20Object%20Reference) (DamageCauser :type Actor%20Object%20Reference))
  (bind _returnvalue (Transformation|GetActorForwardVector DamageCauser))
  (bind _mesh (Variables|Character|GetMesh))
  (bind _returnvalue_2 (* _returnvalue 5e+03))
  (Game|SpawnActorfromClass "/Game/Widgets/BP_Damage.BP_Damage_C" (Transformation|GetActorTransform) "Undefined" "MultiplyWithRoot" 0 Damage 0)
  (Utilities|FlowControl|Sequence
    (:then_0
      (bind _output_get (Variables|Default|SetHealth (- (Variables|Default|GetHealth) Damage)))
      (Components|Activation|Activate (Variables|Default|GetNS_OmniBlood) true)
      (if (<= _output_get 0.0)
        (Collision|SetCollisionProfileName _mesh "Ragdoll" true :!class /Script/Engine.PrimitiveComponent)
        (Physics|SetSimulatePhysics _mesh true)
        (Utilities|FlowControl|Sequence
          (:then_0
            (Physics|AddImpulse _mesh (Math|Vector|MakeVector (.x _returnvalue_2) (.y _returnvalue_2) 0.0) "None" true)
            (Components|DestroyComponent (Variables|Collision|GetCapsuleComponent))
            (Utilities|FlowControl|Delay 3.0)
            (Components|DestroyComponent (Variables|Character|GetMesh)))
          (:then_1
            (Utilities|FlowControl|DoOnce false
              (:Completed
                (bind _asbp_first_person_game_mode (Utilities|Casting|CastToBP_FirstPersonGameMode (Game|GetGameMode)))
                (Variables|/Game/FirstPerson/Blueprints/BP_FirstPersonGameMode.BP_FirstPersonGameMode_C|SetEnemyDeathCount _asbp_first_person_game_mode (+ (Variables|/Game/FirstPerson/Blueprints/BP_FirstPersonGameMode.BP_FirstPersonGameMode_C|GetEnemyDeathCount _asbp_first_person_game_mode) 1))
                (Development|PrintString (Utilities|String|ToString(Integer) (+ (Variables|/Game/FirstPerson/Blueprints/BP_FirstPersonGameMode.BP_FirstPersonGameMode_C|GetEnemyDeathCount _asbp_first_person_game_mode) 1)))))))))
    (:then_1
      (Camera|SetFieldOfView (Variables|/Game/FirstPerson/Blueprints/BP_FirstPersonCharacter.BP_FirstPersonCharacter_C|GetFirstPersonCamera (Variables|Default|GetAs%20BP%20First%20Person%20Character)) (Variables|Default|GetStart%20Field%20Of%20View))
      (bind _fovfloat (Timeline|FOV Play)
        (:Update
          (Camera|SetFieldOfView (Variables|/Game/FirstPerson/Blueprints/BP_FirstPersonCharacter.BP_FirstPersonCharacter_C|GetFirstPersonCamera (Variables|Default|GetAs%20BP%20First%20Person%20Character)) (Math|Float|Lerp (Variables|Default|GetStart%20Field%20Of%20View) 9e+01 _fovfloat)))))))

(event EventBeginPlay
  (bind _asbp_first_person_character (Utilities|Casting|CastToBP_FirstPersonCharacter (Game|GetPlayerCharacter 0)))
  (Variables|Default|SetAs%20BP%20First%20Person%20Character _asbp_first_person_character)
  (bind _randomlocation (Class|NavigationSystemV1|GetRandomLocationinNavigableRadius (Transformation|GetActorLocation) (Variables|Default|GetRadius) 0 0 :!label _label))
  (AI|AIMoveTo self _randomlocation 0 5.0 false
    (:then
      _)
    (:OnFail
      _))
  (Utilities|FlowControl|Delay (Variables|Default|GetDuration))
  (if (not (Variables|Default|GetCanSeePlayer))
    (goto _label)))

(fn ConstructionScript)