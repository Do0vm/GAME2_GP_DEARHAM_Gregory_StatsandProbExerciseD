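; Spitter zombie enemy that roams random navmesh points until pawn sensing spots the player.
; On sight it screams once and approaches, then spawns a projectile, playing vomit FX at close range before resuming roaming.
; Touching the player while aggroed deals contact damage.
; Taking damage spawns a damage actor, bleeds and tweens the player camera's FOV; death ragdolls it with an impulse, then destroys it.
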(event OnSeePawn(ZombieSensing)
  (params (Pawn :type Pawn%20Object%20Reference))
  (bind _as_bp_top_down_character (Variables|Default|GetAs%20BP%20Top%20Down%20Character))
  (if (== Pawn (Variables|Default|GetAs%20BP%20Top%20Down%20Character))
    (Variables|Default|SetCanSeePlayer true)
    (Utilities|FlowControl|Sequence
      (:then_0
        (AI|AIMoveTo self "0, 0, 0" _as_bp_top_down_character (Variables|Default|GetRadius) false
          (:then
            (Transformation|SetActorRotation (Math|Rotator|FindLookatRotation (Transformation|GetActorLocation) (Transformation|GetActorLocation _as_bp_top_down_character)))
            (bind _returnvalue (Game|SpawnActorfromClass "/Game/MillAssets/Zombie/BP_ZombieProjectile.BP_ZombieProjectile_C" (Transformation|GetWorldTransform (Variables|Default|GetProjectileSpawner)) "Undefined" "MultiplyWithRoot" 0 0))
            (if (<= (Math|Vector|Distance(Vector) (Transformation|GetActorLocation) (Transformation|GetActorLocation (Variables|Default|GetAs%20BP%20Top%20Down%20Character))) 6e+02)
              (Components|Activation|Activate (Variables|Default|GetNS_Vomit) (Variables|Default|GetCanSeePlayer))
              (Utilities|FlowControl|Delay 0.5)
              (Actor|DestroyActor _returnvalue)
              (Utilities|FlowControl|RetriggerableDelay 3.0)
              (CallFunction|RoamingMapAI)))))
      (:then_1
        (Utilities|FlowControl|DoOnce false
          (:Completed
            (Audio|PlaySoundatLocation "/Game/Sound/Zombie/DemonScream.DemonScream" (Transformation|GetActorLocation) "0, 0, 0" 1.0 1.0 0.0 0 0 0 0)))))
    (else
      (Variables|Default|SetCanSeePlayer false)
      (Components|Activation|Deactivate (Variables|Default|GetNS_Vomit)))))

(event OnComponentHit(CapsuleComponent)
  (params (HitComponent :type Primitive%20Component%20Object%20Reference) (OtherActor :type Actor%20Object%20Reference) (OtherComp :type Primitive%20Component%20Object%20Reference) (NormalImpulse :type Vector :default "0, 0, 0") (Hit :type Hit%20Result%20Structure%20%28by%20ref%29))
  (bind _as_bp_top_down_character (Variables|Default|GetAs%20BP%20Top%20Down%20Character))
  (if (== OtherActor _as_bp_top_down_character)
    (if (Variables|Default|GetCanSeePlayer)
      (Game|Damage|ApplyDamage _as_bp_top_down_character 2.0 0 self))))

(event Custom|RoamingMapAI
  (Components|Activation|Deactivate (Variables|Default|GetNS_Vomit))
  (bind _randomlocation (Class|NavigationSystemV1|GetRandomLocationinNavigableRadius (Transformation|GetActorLocation) (Variables|Default|GetRadius) 0 0 :!label _label))
  (AI|AIMoveTo self _randomlocation 0 5.0 false
    (:then
      _)
    (:OnFail
      _))
  (Utilities|FlowControl|Delay (Variables|Default|GetDuration))
  (if (not (Variables|Default|GetCanSeePlayer))
    (goto _label)))

(event Game|Damage|EventAnyDamage
  (params (Damage :type Float%20%28single-precision%29) (DamageType :type Damage%20Type%20Object%20Reference) (InstigatedBy :type Controller%20Object%20Reference) (DamageCauser :type Actor%20Object%20Reference))
  (bind _returnvalue (Transformation|GetActorForwardVector DamageCauser))
  (bind _mesh (Variables|Character|GetMesh))
  (bind _returnvalue_2 (* _returnvalue 5e+03))
  (Game|SpawnActorfromClass "/Game/Widgets/BP_Damage.BP_Damage_C" (Transformation|GetActorTransform) "Undefined" "MultiplyWithRoot" 0 Damage 0)
  (Utilities|FlowControl|Sequence
    (:then_0
      (bind _output_get (Variables|Default|SetHealth (- (Variables|Default|GetHealth) Damage)))
      (Components|Activation|Activate (Variables|Default|GetNS_OmniBlood) true)
      (if (<= _output_get 0.0)
        (Components|DestroyComponent (Variables|Collision|GetCapsuleComponent))
        (Collision|SetCollisionProfileName _mesh "Ragdoll" true :!class /Script/Engine.PrimitiveComponent)
        (Physics|SetSimulatePhysics _mesh true)
        (Physics|AddImpulse _mesh (Math|Vector|MakeVector (.x _returnvalue_2) (.y _returnvalue_2) 0.0) "None" true)
        (Utilities|FlowControl|Delay 3.0)
        (Actor|DestroyActor)))
    (:then_1
      (Camera|SetFieldOfView (Variables|/Game/TopDown/Blueprints/BP_TopDownCharacter.BP_TopDownCharacter_C|GetCamera (Variables|Default|GetAs%20BP%20Top%20Down%20Character)) (Variables|Default|GetStart%20Field%20Of%20View))
      (bind _fovfloat (Timeline|Timeline Play)
        (:Update
          (Camera|SetFieldOfView (Variables|/Game/TopDown/Blueprints/BP_TopDownCharacter.BP_TopDownCharacter_C|GetCamera (Variables|Default|GetAs%20BP%20Top%20Down%20Character)) (Math|Float|Lerp (Variables|Default|GetStart%20Field%20Of%20View) 55.0 _fovfloat)))))))

(event EventBeginPlay
  (Components|Activation|Deactivate (Variables|Default|GetNS_Vomit))
  (bind _asbp_top_down_character (Utilities|Casting|CastToBP_TopDownCharacter (Game|GetPlayerCharacter 0)))
  (Variables|Default|SetAs%20BP%20Top%20Down%20Character _asbp_top_down_character)
  (bind _randomlocation (Class|NavigationSystemV1|GetRandomLocationinNavigableRadius (Transformation|GetActorLocation) (Variables|Default|GetRadius) 0 0 :!label _label))
  (AI|AIMoveTo self _randomlocation 0 5.0 false
    (:then
      _)
    (:OnFail
      _))
  (Utilities|FlowControl|Delay (Variables|Default|GetDuration))
  (if (not (Variables|Default|GetCanSeePlayer))
    (goto _label)))

(fn ConstructionScript)