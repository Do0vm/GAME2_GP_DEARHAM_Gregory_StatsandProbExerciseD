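; BP_ZombieProjectile is a short-lived zombie attack projectile that hurts the top-down player character.
; On BeginPlay it caches the player character and destroys itself after a brief delay.
; When its collision component overlaps that player, it applies a small amount of damage and triggers controller force feedback plus a vomit camera shake.
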(event OnComponentBeginOverlap(ZombieProjectileCollision)
  (params (OverlappedComponent :type Primitive%20Component%20Object%20Reference) (OtherActor :type Actor%20Object%20Reference) (OtherComp :type Primitive%20Component%20Object%20Reference) (OtherBodyIndex :type Integer) (bFromSweep :type Boolean) (SweepResult :type Hit%20Result%20Structure%20%28by%20ref%29))
  (bind _returnvalue (Game|GetPlayerController 0))
  (bind _as_bp_top_down_character (Variables|Default|GetAs%20BP%20Top%20Down%20Character))
  (if (== OtherActor _as_bp_top_down_character)
    (Game|Damage|ApplyDamage _as_bp_top_down_character 0.5 0 self)
    (Game|Feedback|ClientPlayForceFeedback _returnvalue "/Game/TopDown/Input/ExplosiveFeedback.ExplosiveFeedback" "None" false false false)
    (Game|Feedback|ClientStartCameraShake _returnvalue "/Game/MillAssets/Camera/BP_VomitCamera.BP_VomitCamera_C" 1.0 "CameraLocal" "0, 0, 0")))

(event EventBeginPlay
  (bind _asbp_top_down_character (Utilities|Casting|CastToBP_TopDownCharacter (Game|GetPlayerCharacter 0)))
  (Variables|Default|SetAs%20BP%20Top%20Down%20Character _asbp_top_down_character)
  (Utilities|FlowControl|Delay 1.0)
  (Actor|DestroyActor))

(fn ConstructionScript)